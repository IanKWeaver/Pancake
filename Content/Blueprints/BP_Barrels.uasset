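; BP_Barrels is a barrel actor that consumes whatever enters its box trigger and rewards the player with score.
; On overlap it destroys the other actor without any type check, waits a second, then spawns a BP_Pancake at an offset high above itself.
; It then casts the player character to BP_ThirdPersonCharacter and adds to its Score.
; An unconnected score-increment fragment is marked for child Blueprints.
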(event `self.Box.OnComponentBeginOverlap`
  (params (OverlappedComponent :type "PrimitiveComponent Object Reference") (OtherActor :type "Actor Object Reference") (OtherComp :type "PrimitiveComponent Object Reference") (OtherBodyIndex :type Integer) (bFromSweep :type Boolean) (SweepResult :type "HitResult Structure (by ref)"))
  (`self.K2_DestroyActor` OtherActor)
  (`KismetSystemLibrary.Delay` 1.0)
  (`|SpawnActorFromClass` "/Game/Blueprints/BP_Pancake.BP_Pancake_C" (`KismetMathLibrary.Conv_VectorToTransform` (+ (`self.K2_GetActorLocation`) (50.0 10.0 470.0))) "Undefined" "OverrideRootScale" null null)
  (bind _asbp_third_person_character (cast `/Game/ThirdPerson/Blueprints/BP_ThirdPersonCharacter` (`GameplayStatics.GetPlayerCharacter` 0)))
  (set `/Game/ThirdPerson/Blueprints/BP_ThirdPersonCharacter.Score` (+ (`/Game/ThirdPerson/Blueprints/BP_ThirdPersonCharacter.Score` _asbp_third_person_character) 10) _asbp_third_person_character))

(fn `UserConstructionScript`)