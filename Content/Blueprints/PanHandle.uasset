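; PanHandle is an actor Blueprint that swings its Panhandle component while something overlaps it.
; Begin overlap plays the RotateLeft timeline, which lerps the component's relative rotation from StartRotation to EndRotation, and end overlap reverses it.
; Overlaps are not filtered by actor.
; RotateRight and Flip timelines drive the same lerp but are never triggered.
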(event `self.ReceiveActorBeginOverlap`
  (params (OtherActor :type "Actor Object Reference"))
  (bind (_direction _rotate_left) (`Timeline|Rotate Left` :!label _label)
    (:`Update`
      (`SceneComponent.K2_SetRelativeRotation` (`self.Panhandle`) (`KismetMathLibrary.RLerp` (`self.StartRotation`) (`self.EndRotation`) _rotate_left) false false))))

(event `self.ReceiveActorEndOverlap`
  (params (OtherActor :type "Actor Object Reference"))
  (goto _label :!via `Reverse`))

(fn `UserConstructionScript`)