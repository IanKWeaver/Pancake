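; Game mode that sets up local multiplayer, with one player for each PlayerStart in the level.
; On BeginPlay it matches numeric PlayerStartTags to player indices, creates a local player and spawns a possessed BP_InputReciever at each matching start, tracking receivers and controllers in arrays.
; SpawnPlayer, not called within this Blueprint, spawns a BP_ThirdPersonCharacter at a given receiver's transform and hands that player's controller to it.
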(event `self.ReceiveBeginPlay`
  (`self.GetPlayerStartPoints`)
  (`self.SpawnInputReceivers`))

(fn `GetPlayerStartPoints`
  (bind _outactors (`GameplayStatics.GetAllActorsOfClass` "/Script/Engine.PlayerStart"))
  (set `self.PlayerStartArray` _outactors))

(fn `NameToInt`
  (params (self2 :type "PlayerStart Object Reference"))
  (returns (ReturnValue :type Integer))
  (return (`KismetStringLibrary.Conv_StringToInt` (`KismetStringLibrary.Conv_NameToString` (`PlayerStart.PlayerStartTag` self2)))))

(fn `SpawnInputReceivers`
  (locals (Index :type Integer))
  (bind _index (`local.Index`))
  (bind _returnvalue (`GameplayStatics.GetPlayerController` (`local.Index`)))
  (for (_ _array_index) (`self.PlayerStartArray`)
    (set `local.Index` _array_index)
    (for _array_element (`self.PlayerStartArray`)
      (if (== (`self.NameToInt` _array_element) (`local.Index`))
        (`GameplayStatics.CreatePlayer` -1)
        (bind _returnvalue_2 (`|SpawnActorFromClass` "/Game/Blueprints/PlayerBP/BP_InputReciever.BP_InputReciever_C" (`self.GetTransform` (`|GetArrayItem` (`self.PlayerStartArray`) _index)) "Undefined" "OverrideRootScale" null _index null))
        (`KismetArrayLibrary.Array_AddUnique` (`self.PlayerInputReceiverArray`) _returnvalue_2)
        (`Controller.Possess` _returnvalue _returnvalue_2)
        (`KismetArrayLibrary.Array_AddUnique` (`self.PlayerControllerArray`) _returnvalue)))))

(fn `SpawnPlayer`
  (params (CurrentPlayerIndex :type Integer) (InputReceiver :type "/Game/Blueprints/PlayerBP/BP_InputReciever Object Reference"))
  (bind _returnvalue (`|SpawnActorFromClass` "/Game/ThirdPerson/Blueprints/BP_ThirdPersonCharacter.BP_ThirdPersonCharacter_C" (`self.GetTransform` InputReceiver) "Undefined" "OverrideRootScale" null CurrentPlayerIndex null))
  (`Controller.Possess` (`GameplayStatics.GetPlayerController` (`local.CurrentPlayerIndex`)) _returnvalue)
  (return))

(fn `UserConstructionScript`)