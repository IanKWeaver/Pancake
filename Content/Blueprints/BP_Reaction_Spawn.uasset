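; BP_Reaction_Spawn is a short-lived actor that shows a floating good or bad reaction with a matching sound.
; On BeginPlay, one random index picks both the W_Reaction element to reveal and the 2D sound, from the set chosen by the Good flag.
; Float then raises the root over a short time with MoveComponentTo and destroys the actor.
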(event `self.ReceiveBeginPlay`
  (bind _reaction (`self.Reaction`))
  (set `self.Reaction` (cast `/Game/UI/W_Reaction` (`WidgetComponent.GetUserWidgetObject` (`self.Widget`)) :!pure true))
  (set `self.Choice` (`KismetMathLibrary.RandomIntegerInRange` 0 2))
  (if (`self.Good?`)
    (`Widget.SetVisibility` (`|GetArrayItem` (`|MakeArray` (`/Game/UI/W_Reaction.Ok` _reaction) (`/Game/UI/W_Reaction.Nice` _reaction) (`/Game/UI/W_Reaction.Tasty` _reaction)) (`self.Choice`)) "Visible")
    (`GameplayStatics.PlaySound2D` (`|GetArrayItem` (`self.GoodSound`) (`self.Choice`)) 1.0 1.0 0.0 null null)
    (else
      (`Widget.SetVisibility` (`|GetArrayItem` (`|MakeArray` (`/Game/UI/W_Reaction.Nasty` _reaction) (`/Game/UI/W_Reaction.Yikes` _reaction) (`/Game/UI/W_Reaction.Meh` _reaction)) (`self.Choice`)) "Visible")
      (`GameplayStatics.PlaySound2D` (`|GetArrayItem` (`self.BadSound`) (`self.Choice`)) 1.0 1.0 0.0 null null)))
  (`self.Float`))

(event `Float`
  (bind _defaultsceneroot (`self.DefaultSceneRoot`))
  (`KismetSystemLibrary.MoveComponentTo` _defaultsceneroot (+ (`SceneComponent.K2_GetComponentLocation` _defaultsceneroot) (0.0 0.0 100.0)) (struct) false false 2.0)
  (`self.K2_DestroyActor`))

(fn `UserConstructionScript`)