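; BP_Barrel is a scoring target that awards its Points value, shown on its text label, when a pancake enters its box.
; The overlap spawns a reaction actor at the pancake, then credits the BP_Pann character matching the pancake's player index and updates its score display.
; It destroys the pancake and, after a short delay, spawns a replacement high above the barrel for the same player.
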(event `self.ReceiveBeginPlay`
  (`TextRenderComponent.K2_SetText` (`self.TextRender`) (`KismetTextLibrary.Conv_IntToText` (`self.Points`))))

(event `self.Box.OnComponentBeginOverlap`
  (params (OverlappedComponent :type "PrimitiveComponent Object Reference") (OtherActor :type "Actor Object Reference") (OtherComp :type "PrimitiveComponent Object Reference") (OtherBodyIndex :type Integer) (bFromSweep :type Boolean) (SweepResult :type "HitResult Structure (by ref)"))
  (bind _asbp_pancake (cast `/Game/Blueprints/BP_Pancake` OtherActor))
  (bind _pancakeplayer (`/Game/Blueprints/BP_Pancake.PancakePlayer` _asbp_pancake))
  (set `self.Pancake Player` _pancakeplayer)
  (`|SpawnActorFromClass` "/Game/Blueprints/BP_Reaction_Spawn.BP_Reaction_Spawn_C" (`KismetMathLibrary.MakeTransform` (`SceneComponent.K2_GetComponentLocation` (`/Game/Blueprints/BP_Pancake.SkeletalMesh` _asbp_pancake))) "Undefined" "OverrideRootScale" null true null)
  (bind _asbp_pann (cast `/Game/Blueprints/BP_Pann` (`GameplayStatics.GetPlayerCharacter` _pancakeplayer)))
  (bind _output_get (set `/Game/Blueprints/BP_Pann.Score` (+ (`/Game/Blueprints/BP_Pann.Score` _asbp_pann) (`self.Points`)) _asbp_pann))
  (set `/Game/UI/W_Ready.Score` (`KismetStringLibrary.Concat_StrStr` "Score: " (`KismetStringLibrary.Conv_IntToString` _output_get)) (`/Game/Blueprints/BP_Pann.Ready` _asbp_pann))
  (`self.K2_DestroyActor` _asbp_pancake)
  (`KismetSystemLibrary.Delay` 1.0)
  (`|SpawnActorFromClass` "/Game/Blueprints/BP_Pancake.BP_Pancake_C" (`KismetMathLibrary.Conv_VectorToTransform` (+ (`self.K2_GetActorLocation` self) (0.0 0.0 800.0))) "Undefined" "OverrideRootScale" null (`self.Pancake Player`) null))

(fn `UserConstructionScript`)