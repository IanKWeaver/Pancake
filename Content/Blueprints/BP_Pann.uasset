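; BP_Pann is a player-controlled pan that creates a per-player ready-up widget and tilts its Panhandle from axis input.
; A one-shot Begin press checks the widget box and increments the GameInstance's Ready count.
; Move axes accumulate clamped flip and turn integers, plus an alternate flip while turned, applied as pitch, roll and yaw.
; Without input, values step back toward zero; turn input of either sign adds in the same direction.
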(event `self.ReceiveBeginPlay`
  ;[1 1 1] Set up Characters and their widgets
  (bind _asplayer_controller (cast `PlayerController` (`self.GetController`) :!label _label))
  (bind _returnvalue (`|CreateWidget` "/Game/UI/W_Ready.W_Ready_C" _asplayer_controller))
  (bind _output_get (set `self.Ready` _returnvalue))
  (`UserWidget.AddToPlayerScreen` _output_get 0))

(event `CustomEvent`
  (params (NewController :type "Controller Object Reference"))
  ;[1 1 1] Set up Characters and their widgets
  (`/Engine/EditorBlueprintResources/StandardMacros.IsValid` (`Controller.K2_GetPawn` NewController)
    (:`Is Valid`
      (goto _label))))

(event `InputAction|Begin`
  (params (Key :type "Key Structure"))
  ;[1 1 1] Ready Up
  (:`Pressed`
    (`/Engine/EditorBlueprintResources/StandardMacros.DoOnce` false
      (:`Completed`
        (`CheckBox.SetCheckedState` (`/Game/UI/W_Ready.CheckBox_0` (`self.Ready`)) "Checked")
        (`/Engine/EditorBlueprintResources/StandardMacros.IncrementInt` (`/Game/Blueprints/PlayerBP/GameInstance.Ready` (cast `/Game/Blueprints/PlayerBP/GameInstance` (`GameplayStatics.GetGameInstance`) :!pure true)))))))

(event `InputAxis|Move Forward / Backward`
  (params (AxisValue :type "Float (single-precision)"))
  (bind _fliprotationold (`self.FlipRotationOld`))
  (bind _altfliprotationold (`self.AltFlipRotationOld`))
  (bind _altfliprotationold_2 (`self.AltFlipRotationOld`))
  (bind _fliprotationold_2 (`self.FlipRotationOld`))
  ;[1 1 1] Actions for Rotations and Flipping
  ;;[0.003125 0.05138 1] Flip
  ;;;[0 0 0] IsInput?
  (if (== AxisValue 0.0)
    ;;;[0 0 0] IsCentered?
    (if (not (== _fliprotationold 0))
      ;;;[0 0 0] - or +?
      (if (< _fliprotationold 0)
        ;;;[0 0 0] Return rotation to 0
        (`/Engine/EditorBlueprintResources/StandardMacros.IncrementInt` _fliprotationold_2
          (:`  `
            _))
        (else
          (`/Engine/EditorBlueprintResources/StandardMacros.DecrementInt` _fliprotationold_2
            (:`  `
              _))))
      ;;;[0.06771 0.06771 0.06771] Same thing except for Alternate flip rotation
      (if (== _altfliprotationold_2 0)
        _
        (elif (< _altfliprotationold_2 0)
          (`/Engine/EditorBlueprintResources/StandardMacros.IncrementInt` _altfliprotationold
            (:`  `
              _))
          (else
            (`/Engine/EditorBlueprintResources/StandardMacros.DecrementInt` _altfliprotationold
              (:`  `
                _)))))
      (`self.OldRotation` :!label _label_2))
    (else
      ;;;[0 0 0] Are both rotations active?
      (if (!= (`self.TurnRotationOld`) 0)
        ;;;[0 0 0] Set AltFlip rotation if so
        (set `self.AltFlipRotationOld` (`KismetMathLibrary.Clamp` (`KismetMathLibrary.FTrunc` (+ (* (stale `InputAxis|Move Right / Left` AxisValue) (`self.FlipSpeedOld`)) (`self.AltFlipRotationOld`))) -30 30)))
      ;;;[0 0 0] Set flip rotation
      (set `self.FlipRotationOld` (`KismetMathLibrary.Clamp` (`KismetMathLibrary.FTrunc` (+ (* AxisValue (`self.FlipSpeedOld`)) (`self.FlipRotationOld`))) -30 30))
      (goto _label_2))))

(event `InputAxis|Move Right / Left`
  (params (AxisValue :type "Float (single-precision)"))
  (bind _turnrotationold (`self.TurnRotationOld`))
  (bind _turnrotationold_2 (`self.TurnRotationOld`))
  ;[1 1 1] Actions for Rotations and Flipping
  ;;[1 0 0.03483] Turn
  (if (== AxisValue 0.0)
    (if (== _turnrotationold_2 0)
      _
      (elif (< _turnrotationold_2 0)
        (`/Engine/EditorBlueprintResources/StandardMacros.IncrementInt` _turnrotationold
          (:`  `
            (goto _label_2)))
        (else
          (`/Engine/EditorBlueprintResources/StandardMacros.DecrementInt` _turnrotationold
            (:`  `
              (goto _label_2))))))
    (else
      ;;;[1 1 1] If Flip up Turn normal otherwise if down invert
      (if (>= (stale `InputAxis|Move Forward / Backward` AxisValue) 0.0)
        (set `self.TurnRotationOld` (`KismetMathLibrary.Clamp` (`KismetMathLibrary.FTrunc` (+ (* AxisValue (`self.TurnSpeedOld`)) (`self.TurnRotationOld`))) -30 30))
        (goto _label_2)
        (else
          (set `self.TurnRotationOld` (`KismetMathLibrary.Clamp` (`KismetMathLibrary.FTrunc` (+ (* (- 0.0 AxisValue) (`self.TurnSpeedOld`)) (`self.TurnRotationOld`))) -30 30))
          (goto _label_2))))))

(event `OldRotation`
  ;[0.9291 0.3051 1] Apply Rotation
  (`SceneComponent.K2_SetRelativeRotation` (`self.Panhandle`) (`KismetMathLibrary.MakeRotator` (`KismetMathLibrary.Conv_IntToDouble` (`self.TurnRotationOld`)) (`KismetMathLibrary.Conv_IntToDouble` (`self.FlipRotationOld`)) (`KismetMathLibrary.Conv_IntToDouble` (`self.AltFlipRotationOld`))) false false))

(fn `RotationOld`)

(fn `UserConstructionScript`)